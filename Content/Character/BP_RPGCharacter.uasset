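; BP_RPGCharacter is a character Blueprint with melee-style attack input, health and ragdoll on death.
; E calls the Attack component, plays a montage and disables movement, using a flag and a fixed delay to block re-triggering before restoring walking.
; The Health component's zero event turns on mesh physics and disables capsule collision, while F subtracts one health.
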(event OnHealthZero(Health)
  (Physics|SetSimulatePhysics (Variables|Character|GetMesh) true)
  (Collision|SetCollisionEnabled (Variables|Default|GetCapsuleComponent) "NoCollision"))

(event Input|KeyboardEvents|E
  (params (Key :type Key%20Structure :default "None"))
  (:Pressed
    (if (not (Variables|Default|GetbIsAttacking))
      (Class|AttackComponent|Attack (Variables|Default|GetAttack))
      (Pawn|Components|CharacterMovement|DisableMovement (Variables|Character|GetCharacterMovement))
      (Variables|Default|SetbIsAttacking true)
      (Animation|PlayAnimMontage "/Game/Character/Assets/AnimMontages/attack_montage.attack_montage" 1.0 "None")
      (Utilities|FlowControl|Delay 0.833333)
      (Pawn|Components|CharacterMovement|SetMovementMode (Variables|Character|GetCharacterMovement) "MOVE_Walking" 0)
      (Variables|Default|SetbIsAttacking false))))

(event Input|KeyboardEvents|F
  (params (Key :type Key%20Structure :default "None"))
  (:Pressed
    (Class|HealthComponent|ChangeHealth (Variables|Default|GetHealth) -1.0)))

(fn ConstructionScript)