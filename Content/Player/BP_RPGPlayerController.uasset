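; Player controller for the RPG that creates the HUD and keeps its inventory and health displays in sync with the player character.
; On BeginPlay it caches the BP_RPGCharacter pawn, adds WBP_HUD to the viewport, then binds to the character's Inventory and Health change events.
; Those events push the corresponding component into the HUD's update functions, so refreshes are event-driven.
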(event EventBeginPlay
  (Utilities|FlowControl|Sequence
    (:then_0
      (bind _asbp_rpgcharacter (Utilities|Casting|CastToBP_RPGCharacter (Game|Player|GetPlayerPawn 0)))
      (Variables|Default|SetAs%20BP%20RPGCharacter _asbp_rpgcharacter))
    (:then_1
      (bind _returnvalue (UserInterface|CreateWidget "/Game/UI/WBP_HUD.WBP_HUD_C"))
      (bind _output_get (Variables|Default|SetHUDRef _returnvalue))
      (UserInterface|Viewport|AddtoViewport _output_get 0))
    (:then_2
      (|BindOnInventoryUpdated))
    (:then_3
      (|BindOnHealthChanged))))

(fn ConstructionScript)

(event Custom|RefreshHUD
  (Default|UpdateInventory (Variables|Default|GetHUDRef) (Variables|/Script/RPG_Game.RPGCharacter|GetInventory (Variables|Default|GetAs%20BP%20RPGCharacter))))

(event Custom|UpdateHealth
  (Default|UpdateHealth (Variables|Default|GetHUDRef) (Variables|/Script/RPG_Game.RPGCharacter|GetHealth (Variables|Default|GetAs%20BP%20RPGCharacter))))