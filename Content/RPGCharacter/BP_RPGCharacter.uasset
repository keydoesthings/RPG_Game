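; BP_RPGCharacter is an RPG character Blueprint wired as a debug test of its Health component.
; Pressing F lowers health by one through the component's ChangeHealth.
; The component's zero, max and changed events print debug strings, and the changed event also prints the current health value.
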(event OnHealthZero(Health)
  (Development|PrintString "zero"))

(event OnHealthMax(Health)
  (Development|PrintString "max"))

(event OnHealthChanged(Health)
  (Development|PrintString "changed")
  (Development|PrintString (Utilities|String|ToString(Float) (Variables|/Script/RPG_Game.HealthComponent|GetCurrentHealth (Variables|Default|GetHealth)))))

(event Input|KeyboardEvents|F
  (params (Key :type Key%20Structure :default "None"))
  (:Pressed
    (Class|HealthComponent|ChangeHealth (Variables|Default|GetHealth) -1.0)))

(fn ConstructionScript)